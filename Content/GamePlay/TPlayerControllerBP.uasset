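; Player controller Blueprint that switches between three formations and adjusts a direction through player input.
; Numpad keys 1 to 3 call OnFormation, which runs UseRemoveComp on the previous formation, applies the new one and stores its index.
; The AddDiraction and MinusDiraction input actions change the direction, then reapply the current formation.
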(event `OnFormation`
  (params (Index :type Integer))
  (`self.UseRemoveComp` (`self.FormationIndex`))
  (`self.UseFormation` Index)
  (set `self.FormationIndex` Index))

(event `Key|NumPadOne`
  (params (Key :type "Key Structure"))
  (:`Pressed`
    (`self.OnFormation` 0)))

(event `Key|NumPadTwo`
  (params (Key :type "Key Structure"))
  (:`Pressed`
    (`self.OnFormation` 1)))

(event `Key|NumPadThree`
  (params (Key :type "Key Structure"))
  (:`Pressed`
    (`self.OnFormation` 2)))

(event `InputAction|AddDiraction`
  (params (Key :type "Key Structure"))
  (:`Pressed`
    (`self.AddDiraction`)
    (`self.OnFormation` (`self.FormationIndex`))))

(event `InputAction|MinusDiraction`
  (params (Key :type "Key Structure"))
  (:`Pressed`
    (`self.MinusDiraction`)
    (`self.OnFormation` (`self.FormationIndex`))))

(fn `UserConstructionScript`)